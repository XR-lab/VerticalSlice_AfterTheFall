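; Generated mesh actor that procedurally builds a snow layer over chosen actors using Geometry Script.
; GenerateMeshCache merges the actors' root component meshes in world space and builds a BVH for raycasts.
; On rebuild, a grid of downward rays places normal-aligned spheres on faces passing the SnowCoverage slope test, then converts them to local space.
; Optional remeshing fuses them through SDF morphology and smoothing, then regenerates planar UVs, tangents and normals.
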(event Custom|GenerateMeshCache
  (DynamicMeshActor|ReleaseAllComputeMeshes)
  (Utilities|FlowControl|Sequence
    (:then_0
      (bind _returnvalue (DynamicMeshActor|AllocateComputeMesh))
      (Variables|Default|SetRaycastMeshActors _returnvalue)
      (for _array_element (Variables|Snow|GenerateSnowSpheres|GetMeshesToAddSnowTo)
        (bind _returnvalue_2 (DynamicMeshActor|AllocateComputeMesh))
        (bind _returnvalue_3 (GeometryScript|Scene|CopyMeshfromComponent :Component (Variables|/Script/Engine.Actor|GetRootComponent _array_element) :ToDynamicMesh _returnvalue_2 :bTransformToWorld true :Debug 0)
          (:Failure
            _)
          (:Success
            (GeometryScript|MeshEdits|AppendMesh :TargetMesh (Variables|Default|GetRaycastMeshActors) :AppendMesh _returnvalue_3 :AppendOptions "(CombineMode=EnableAllMatching)" :Debug 0)))
        (Class|DynamicMeshActor|ReleaseComputeMesh _returnvalue_2)))
    (:then_1
      (bind (_outputbvh _returnvalue_4) (Class|GeometryScriptLibraryMeshSpatial|BuildBVHforMesh (Variables|Default|GetRaycastMeshActors) 0))
      (Variables|Default|SetOutput%20BVH _outputbvh))))

(event Custom|ReleaseComputeMeshes
  (DynamicMeshActor|ReleaseAllComputeMeshes))

(event EventBeginPlay)

(event Collision|EventActorBeginOverlap
  (params (OtherActor :type Actor%20Object%20Reference)))

(event EventTick
  (params (DeltaSeconds :type Float%20%28single-precision%29)))

(event Events|EventOnRebuildGeneratedMesh
  (params (TargetMesh :type Dynamic%20Mesh%20Object%20Reference))
  (Variables|Default|SetTarget%20Mesh TargetMesh)
  (if (Variables|Snow|GenerateSnowSpheres|GetGenerateSnow)
    (Utilities|FlowControl|Sequence
      (:then_0
        (for _index (range 0 (Math|Float|Round (/ (- (.x (.max (Class|GeometryScriptLibraryMeshQueryFunctions|GetMeshBoundingBox (stale Custom|GenerateMeshCache _returnvalue_4)))) (.x (.min (Class|GeometryScriptLibraryMeshQueryFunctions|GetMeshBoundingBox (stale Custom|GenerateMeshCache _returnvalue_4))))) (Variables|Snow|GenerateSnowSpheres|GetGridSpacing))))
          (for _index_2 (range 0 (Math|Float|Round (/ (- (.y (.max (Class|GeometryScriptLibraryMeshQueryFunctions|GetMeshBoundingBox (stale Custom|GenerateMeshCache _returnvalue_4)))) (.y (.min (Class|GeometryScriptLibraryMeshQueryFunctions|GetMeshBoundingBox (stale Custom|GenerateMeshCache _returnvalue_4))))) (Variables|Snow|GenerateSnowSpheres|GetGridSpacing))))
            (bind _hitresult (Class|GeometryScriptLibraryMeshSpatial|FindNearestRayIntersectionwithMesh :TargetMesh (Variables|Default|GetRaycastMeshActors) :QueryBVH (Variables|Default|GetOutput%20BVH) :RayOrigin (Math|Vector|MakeVector (+ (.x (.min (Class|GeometryScriptLibraryMeshQueryFunctions|GetMeshBoundingBox (stale Custom|GenerateMeshCache _returnvalue_4)))) (* _index (Variables|Snow|GenerateSnowSpheres|GetGridSpacing))) (+ (* _index_2 (Variables|Snow|GenerateSnowSpheres|GetGridSpacing)) (.y (.min (Class|GeometryScriptLibraryMeshQueryFunctions|GetMeshBoundingBox (stale Custom|GenerateMeshCache _returnvalue_4))))) (+ (- (.z (.max (Class|GeometryScriptLibraryMeshQueryFunctions|GetMeshBoundingBox (stale Custom|GenerateMeshCache _returnvalue_4)))) (.z (.min (Class|GeometryScriptLibraryMeshQueryFunctions|GetMeshBoundingBox (stale Custom|GenerateMeshCache _returnvalue_4))))) 1e+02)) :RayDirection "0.000000,0.000000,-1.000000" :Debug 0)
              (:Found
                (if (>= (.z (.ReturnValue (Class|GeometryScriptLibraryMeshQueryFunctions|GetTriangleFaceNormal (Variables|Default|GetRaycastMeshActors) (.hittriangleid _hitresult)))) (Math|Float|Absolute(Float) (- (Variables|Snow|GenerateSnowSpheres|GetSnowCoverage) 1.0)))
                  (Class|GeometryScriptLibraryMeshPrimitiveFunctions|AppendSphereBox :TargetMesh (Variables|Default|GetTarget%20Mesh) :Transform (Math|Transform|MakeTransform (.hitposition _hitresult) (Math|Rotator|MakeRotfromZ (Math|Vector|MakeVector (.x (.ReturnValue (Class|GeometryScriptLibraryMeshQueryFunctions|GetTriangleFaceNormal (Variables|Default|GetRaycastMeshActors) (.hittriangleid _hitresult)))) (.y (.ReturnValue (Class|GeometryScriptLibraryMeshQueryFunctions|GetTriangleFaceNormal (Variables|Default|GetRaycastMeshActors) (.hittriangleid _hitresult)))) (.z (.ReturnValue (Class|GeometryScriptLibraryMeshQueryFunctions|GetTriangleFaceNormal (Variables|Default|GetRaycastMeshActors) (.hittriangleid _hitresult)))))) (Math|Vector|MakeVector 1.0 1.0 (Variables|Snow|GenerateSnowSpheres|GetSnowSphereScaleX))) :Radius (Variables|Snow|GenerateSnowSpheres|GetSphereRadius) :Debug 0)))))))
      (:then_1
        (GeometryScript|Transforms|TransformMesh (Variables|Default|GetTarget%20Mesh) (Math|Transform|InvertTransform (Transformation|GetActorTransform)) true 0))
      (:then_2
        (if (Variables|Snow|GenerateSnowMesh|GetRemesh)
          (bind _returnvalue (Class|GeometryScriptLibraryMeshVoxelFunctions|ApplyMeshMorphology (Variables|Default|GetTarget%20Mesh) (Utilities|Struct|MakeGeometryScriptMorphologyOptions (Utilities|Struct|MakeGeometryScript3DGridParameters "GridCellSize" (Variables|Snow|GenerateSnowMesh|GetGridCellSize) 64) false (Utilities|Struct|MakeGeometryScript3DGridParameters "GridResolution" 0.5 64) "Dilate" (Variables|Snow|GenerateSnowMesh|GetSnowThickness)) 0))
          (bind _returnvalue_2 (Class|GeometryScriptLibraryMeshDeformFunctions|ApplyIterativeSmoothingtoMesh :TargetMesh _returnvalue :Options (Utilities|Struct|MakeGeometryScriptIterativeMeshSmoothingOptions (Variables|Snow|GenerateSnowMesh|GetSmoothIterations) 0.2 "FullMeshSelection") :Debug 0))
          (Class|GeometryScriptLibraryMeshUVFunctions|SetMeshUVsfromPlanarProjection :TargetMesh _returnvalue_2 :PlaneTransform (Math|Transform|MakeTransform "0, 0, 0" "0, 0, 0" (Math|Vector|MakeVector (Math|Float|Max(Float) (.x (- (.max (Class|GeometryScriptLibraryMeshQueryFunctions|GetMeshBoundingBox _returnvalue_2)) (.min (Class|GeometryScriptLibraryMeshQueryFunctions|GetMeshBoundingBox _returnvalue_2)))) (.y (- (.max (Class|GeometryScriptLibraryMeshQueryFunctions|GetMeshBoundingBox _returnvalue_2)) (.min (Class|GeometryScriptLibraryMeshQueryFunctions|GetMeshBoundingBox _returnvalue_2))))) (Math|Float|Max(Float) (.x (- (.max (Class|GeometryScriptLibraryMeshQueryFunctions|GetMeshBoundingBox _returnvalue_2)) (.min (Class|GeometryScriptLibraryMeshQueryFunctions|GetMeshBoundingBox _returnvalue_2)))) (.y (- (.max (Class|GeometryScriptLibraryMeshQueryFunctions|GetMeshBoundingBox _returnvalue_2)) (.min (Class|GeometryScriptLibraryMeshQueryFunctions|GetMeshBoundingBox _returnvalue_2))))) (Math|Float|Max(Float) (.x (- (.max (Class|GeometryScriptLibraryMeshQueryFunctions|GetMeshBoundingBox _returnvalue_2)) (.min (Class|GeometryScriptLibraryMeshQueryFunctions|GetMeshBoundingBox _returnvalue_2)))) (.y (- (.max (Class|GeometryScriptLibraryMeshQueryFunctions|GetMeshBoundingBox _returnvalue_2)) (.min (Class|GeometryScriptLibraryMeshQueryFunctions|GetMeshBoundingBox _returnvalue_2))))))) :Debug 0)
          (bind _returnvalue_3 (Class|GeometryScriptLibraryMeshNormalsFunctions|ComputeTangents :Debug 0))
          (Class|GeometryScriptLibraryMeshNormalsFunctions|ComputeSplitNormals :TargetMesh _returnvalue_3 :SplitOptions (Utilities|Struct|MakeGeometryScriptSplitNormalsOptions true 8e+01 false "(bDefaultLayer=True,ExtendedLayerIndex=0)") :Debug 0))))))

(fn ConstructionScript)