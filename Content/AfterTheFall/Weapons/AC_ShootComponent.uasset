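; Weapon shooting component that fires a hitscan shot from a given scene component along its forward vector using a short-range Visibility line trace.
; On a hit, it plays a sound and Niagara effect chosen by physical surface type and spawns a temporary bullet-hole decal.
; Hit actors implementing the BI_Hittable interface receive OnHit with damage, impact point and normal-based rotation, leaving the reaction to the target.
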(event Custom|ShootRaycast
  (params (ShootLocation :type Static%20Mesh%20Component%20Object%20Reference))
  (bind _returnvalue (Transformation|GetWorldLocation ShootLocation))
  ;[1 1 1] Active a Raycast
  (bind (_outhit _returnvalue_2) (Collision|LineTraceByChannel _returnvalue (+ _returnvalue (* (Math|Vector|GetForwardVector (Transformation|GetWorldRotation ShootLocation)) 1.5e+03)) "TraceTypeQuery1" false 0 "None"))
  (if _returnvalue_2
    (CallFunction|PlayImpactSound (Variables|/Script/PhysicsCore.PhysicalMaterial|GetSurfaceType (.PhysMat (Collision|BreakHitResult _outhit))) (.Location (Collision|BreakHitResult _outhit)))
    (Rendering|Decal|SpawnDecalatLocation "/Game/AfterTheFall/ParticleSystems/BulletImpact/M_bulletImpact_Decal.M_bulletImpact_Decal" "2.000000,2.000000,2.000000" (.Location (Collision|BreakHitResult _outhit)) (Math|Rotator|MakeRotationfromAxes (.ImpactNormal (Collision|BreakHitResult _outhit)) (.ImpactNormal (Collision|BreakHitResult _outhit)) (.ImpactNormal (Collision|BreakHitResult _outhit))) 14.0)
    (bind _asbi_hittable (Utilities|Casting|CastToBI_Hittable (.HitActor (Collision|BreakHitResult _outhit))))
    (Default|OnHit _asbi_hittable (Variables|Default|GetDamage) (.ImpactPoint (Collision|BreakHitResult _outhit)) (Math|Rotator|MakeRotationfromAxes (.ImpactNormal (Collision|BreakHitResult _outhit)) (.ImpactNormal (Collision|BreakHitResult _outhit)) (.ImpactNormal (Collision|BreakHitResult _outhit))))))

(fn PlayImpactSound
  (params (Physics%20Mat :type EPhysicalSurface%20Enum :default "SurfaceType_Default") (Impact%20Pos :type Vector))
  (bind _returnvalue (Audio|SpawnSoundatLocation (Utilities|Select :Index Physics%20Mat :SurfaceType_Default "/Game/AfterTheFall/Audio/SFX/BulletImpactSFX/Snow/MS_BulletSnowImpactSound.MS_BulletSnowImpactSound" :SurfaceType1 "/Game/AfterTheFall/Audio/SFX/BulletImpactSFX/Snow/MS_BulletSnowImpactSound.MS_BulletSnowImpactSound" :SurfaceType2 "/Game/AfterTheFall/Audio/SFX/BulletImpactSFX/Concrete/MS_BulletConcreteImpactSound.MS_BulletConcreteImpactSound" :SurfaceType3 "/Game/AfterTheFall/Audio/SFX/BulletImpactSFX/Glass/MS_BulletGlassImpactSound.MS_BulletGlassImpactSound" :SurfaceType4 "/Game/AfterTheFall/Audio/SFX/BulletImpactSFX/Metal/MS_BulletMetalImpactSound.MS_BulletMetalImpactSound") Impact%20Pos "0, 0, 0" 1.0 1.0 0.0 0 0))
  (Niagara|SpawnSystematLocation (Utilities|Select :Index Physics%20Mat :SurfaceType_Default 0 :SurfaceType1 "/Game/AfterTheFall/ParticleSystems/MaterialParticles/SnowImpact/FXS_SnowImpact.FXS_SnowImpact" :SurfaceType2 "/Game/AfterTheFall/ParticleSystems/MaterialParticles/ConcreteImpact/FXS_ConcreteImpact.FXS_ConcreteImpact" :SurfaceType3 "/Game/AfterTheFall/ParticleSystems/MaterialParticles/GlassImpact/FXS_GlassImpact.FXS_GlassImpact" :SurfaceType4 "/Game/AfterTheFall/ParticleSystems/MaterialParticles/MetalImpact/FXS_MetalImpact.FXS_MetalImpact") Impact%20Pos)
  (Utilities|IsValid _returnvalue
    (:Is%20Valid
      (Audio|Components|Audio|StopDelayed _returnvalue 1.0))))