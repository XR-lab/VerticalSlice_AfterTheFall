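; VR grenade that can be stored, grabbed and armed or disarmed with the holding hand's trigger to damage zombies.
; Grabbing adds that hand's weapon input context, and the trigger toggles the active state and enables Tick.
; Tick drives BPGrenadeSFXComponent's beep countdown, which also times the blinking point light.
; On detonation it hits overlapping BP_Zombie actors through BI_Hittable, hides the mesh, plays the effect and destroys itself after a delay.
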(event OnGrabbed(GrabComponentSnap)
  ;[1 1 1] When the Grenade is grabbed, enable input and add the Grenade Input Mapping Context. Disable and remove when the Grenade is dropped.
  (Input|EnableInput (Game|GetPlayerController 0))
  (Input|AddMappingContext (PlayerController|LocalPlayerSubsystems|GetEnhancedInputLocalPlayerSubsystem (Game|GetPlayerController 0)) (select (Utilities|Enum|Equal(Enum) (Default|GetHeldbyHand (Variables|Default|GetGrabComponentSnap)) "Right") "/Game/VRTemplate/Input/IMC_Weapon_Right.IMC_Weapon_Right" "/Game/VRTemplate/Input/IMC_Weapon_Left.IMC_Weapon_Left") 0 "(bIgnoreAllPressedKeysUntilRelease=True,bForceImmediately=False)"))

(event OnDropped(GrabComponentSnap)
  ;[1 1 1] When the Grenade is grabbed, enable input and add the Grenade Input Mapping Context. Disable and remove when the Grenade is dropped.
  (Input|DisableInput (Game|GetPlayerController 0))
  (Input|RemoveMappingContext (PlayerController|LocalPlayerSubsystems|GetEnhancedInputLocalPlayerSubsystem (Game|GetPlayerController 0)) (select (Utilities|Enum|Equal(Enum) (Default|GetHeldbyHand (Variables|Default|GetGrabComponentSnap)) "Right") "/Game/VRTemplate/Input/IMC_Weapon_Right.IMC_Weapon_Right" "/Game/VRTemplate/Input/IMC_Weapon_Left.IMC_Weapon_Left") "(bIgnoreAllPressedKeysUntilRelease=True,bForceImmediately=False)"))

(event Input|EnhancedActionEvents|EnhancedInputActionIA_Shoot_Right
  (params (ActionValue :type Boolean) (ElapsedSeconds :type Float%20%28double-precision%29) (TriggeredSeconds :type Float%20%28double-precision%29) (InputAction :type Input%20Action%20Object%20Reference :default "/Game/VRTemplate/Input/Actions/IA_Shoot_Right.IA_Shoot_Right"))
  ;[1 1 1] When the grenade is grabbed and you press the trigger the grenade will be set active
  (:Started
    (if (Utilities|Enum|Equal(Enum) (Default|GetHeldbyHand (Variables|Default|GetGrabComponentSnap)) "Right")
      (CallFunction|ActivateGrenade)
      (Actor|Tick|SetActorTickEnabled true))))

(event Input|EnhancedActionEvents|EnhancedInputActionIA_Shoot_Left
  (params (ActionValue :type Boolean) (ElapsedSeconds :type Float%20%28double-precision%29) (TriggeredSeconds :type Float%20%28double-precision%29) (InputAction :type Input%20Action%20Object%20Reference :default "/Game/VRTemplate/Input/Actions/IA_Shoot_Left.IA_Shoot_Left"))
  ;[1 1 1] When the grenade is grabbed and you press the trigger the grenade will be set active
  (:Started
    (if (Utilities|Enum|Equal(Enum) (Default|GetHeldbyHand (Variables|Default|GetGrabComponentSnap)) "Left")
      (CallFunction|ActivateGrenade)
      (Actor|Tick|SetActorTickEnabled true))))

(event EventBeginPlay
  (Default|SetupStorableComponent (Variables|Default|GetAC_StoreableComponent) (Variables|Default|GetSM_Granade)))

(event EventTick
  (params (DeltaSeconds :type Float%20%28single-precision%29))
  ;[1 1 1] Update Loop
  (bind _explotion (Default|PlayGrenadeDetonation (Variables|Default|GetBP_GrenadeSFX_Component) DeltaSeconds))
  (if _explotion
    ;;[1 1 1] explosion
    (CallFunction|PlayExplosion)
    (Utilities|FlowControl|Delay 3.0)
    (Actor|DestroyActor)
    (elif (Variables|Default|GetIsActive)
      (CallFunction|ActiveteLight)
      (if (not (Variables|/Game/AfterTheFall/Audio/SFX/GrenadeSFX/BP_GrenadeSFX_Component.BP_GrenadeSFX_Component_C|GetgrenadeActivated (Variables|Default|GetBP_GrenadeSFX_Component)))
        ;;[1 1 1] Starts the timers wen the the Grenade is active
        (Default|SetupEvent (Variables|Default|GetBP_GrenadeSFX_Component) (Variables|Default|GetIsActive) 4 0.5 1.0 0.9 (Variables|Default|GetMS_GrenadeSound)))
      (else
        ;;[1 1 1] Stops all the Timers wen the Grenade get deactived
        (Utilities|Time|ClearTimerbyFunctionName 0 "ChangeMaterial")
        (Utilities|Time|ClearandInvalidateTimerbyHandle (Variables|Default|GetExplosionTimerHandle))
        (Default|SetupEvent (Variables|Default|GetBP_GrenadeSFX_Component) (Variables|Default|GetIsActive) 0 0.0 (Variables|Default|GetTimeTillExpotion) 0.0 (Variables|Default|GetMS_GrenadeSound))
        (Actor|Tick|SetActorTickEnabled false)))))

(fn ConstructionScript)

(fn ActivateGrenade
  (Variables|Default|SetIsActive (not (Variables|Default|GetIsActive)))
  (return))

(fn ActiveteLight
  (bind _pointlight (Variables|Default|GetPointLight))
  (Math|Float|CompareFloat (Variables|/Game/AfterTheFall/Audio/SFX/GrenadeSFX/BP_GrenadeSFX_Component.BP_GrenadeSFX_Component_C|GetdelayTillBeep (Variables|Default|GetBP_GrenadeSFX_Component)) 0.1
    (:>
      (Rendering|Components|Light|SetIntensity _pointlight 0.0))
    (:==
      (Rendering|Components|Light|SetIntensity _pointlight 5e+03 :!label _label))
    (:<
      (goto _label)))
  (return))

(fn CastExplosionSphere
  (for _array_element (Collision|GetOverlappingActors (Variables|Default|GetExpotionSphere) "/Game/AfterTheFall/Enemies/BP_Zombie.BP_Zombie_C" :!class /Script/Engine.PrimitiveComponent)
    ;[1 1 1] BI_Hitable
    (bind _asbi_hittable (Utilities|Casting|CastToBI_Hittable _array_element))
    (Default|OnHit _asbi_hittable (Variables|Default|GetDamage) "0, 0, 0" "0, 0, 0"))
  (return))

(fn PlayExplosion
  (if (Variables|Default|GetIsActive)
    (CallFunction|CastExplosionSphere)
    (Rendering|SetVisibility (Variables|Default|GetSM_Granade) false false)
    (Rendering|Components|Light|SetIntensity (Variables|Default|GetPointLight) 0.0)
    (Components|Activation|Activate (Variables|Default|GetFXS_GrenadeExplosion) true)
    (Variables|Default|SetIsActive false)))