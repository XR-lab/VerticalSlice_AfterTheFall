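; BP_Spawnpoint is a zombie spawn location that scores itself through an interest weight, likely for choosing where to spawn.
; GetWeight lowers that weight by the player's horizontal distance, scaled by DistanceWeight, and by the number of zombies GetZombieCount finds within SpawnRegionSize.
; Each call subtracts from the current weight and clears the zombie count, while ResetWeight sets the weight back to zero.
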(event Custom|GetWeight
  ;[1 1 1] Calculate the distance between the spawnpoint and the player.
  (bind _returnvalue (Actor|GetActorOfClass (Variables|Default|GetPlayer)))
  ;[1 1 1] Subtract the distance and the zombie count from the interest weight.
  (CallFunction|GetZombieCount)
  ;[1 1 1] Set the interest weight and reset the zombie count.
  (Variables|Default|SetInterestWeight (- (- (Variables|Default|GetInterestWeight) (/ (Math|Vector|VectorLengthXY (- (Transformation|GetActorLocation) (Transformation|GetActorLocation _returnvalue))) (Variables|Default|GetDistanceWeight))) (Variables|Default|GetZombieCount)))
  (Variables|Default|SetZombieCount 0))

(event Custom|ResetWeight
  ;[1 1 1] Reset interest weight on activation.
  (Variables|Default|SetInterestWeight 0.0))

(event Custom|GetZombieCount
  ;[1 1 1] Calculate the distance of every zombie towards the spawnpoint.
  (bind _outactors (Actor|GetAllActorsOfClass (Variables|Default|GetZombie)))
  (for _array_element _outactors
    ;[1 1 1] If a zombie is within the region size, add one to the zombie count.
    (if (<= (Math|Vector|Distance(Vector) (Transformation|GetActorLocation) (Transformation|GetActorLocation _array_element)) (Variables|Default|GetSpawnRegionSize))
      (bind _result (Math|Integer|IncrementInt (Variables|Default|GetZombieCount))
        (:%20%20
          (Variables|Default|SetZombieCount _result))))))

(fn ConstructionScript)