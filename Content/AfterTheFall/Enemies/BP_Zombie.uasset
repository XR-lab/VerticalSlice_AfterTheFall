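; Enemy zombie that detects the VR player with a vision sphere, setting it as the AI blackboard target.
; Attack triggers animation and sound, while Tick sphere-traces the right hand whenever CheckSphere is set to damage the player.
; Hits always spawn blood effects, adding decals, health damage and a flinch montage while alive.
; The health component's death event ends AI, enables ragdoll physics and destroys the actor after a delay.
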(event OnDeath(AC_HealthComponent)
  ;[1 1 1] When the zombie is dead, start a delay before destroying the zombie
  (Class|AudioParameterControllerInterface|SetTriggerParameter (Variables|Default|GetMS_ZombieSoundEffects) "DeathEffect")
  (bind _asaic_zombie (Utilities|Casting|CastToAIC_Zombie (AI|GetAIController self)))
  (Default|EndAI _asaic_zombie)
  (bind _asabp_zombie_ (Utilities|Casting|CastToABP_Zombie_ (Components|SkeletalMesh|GetAnimInstance (Variables|Character|GetMesh))))
  (Variables|/Game/AfterTheFall/Enemies/ABP_Zombie_.ABP_Zombie__C|SetbDead _asabp_zombie_ true)
  (Variables|Default|SetbDead true)
  (Physics|SetSimulatePhysics (Variables|Character|GetMesh) true)
  (Utilities|FlowControl|Delay 3e+01)
  (Actor|DestroyActor))

(event OnComponentBeginOverlap(VisionSphere)
  (params (OverlappedComponent :type Primitive%20Component%20Object%20Reference) (OtherActor :type Actor%20Object%20Reference) (OtherComp :type Primitive%20Component%20Object%20Reference) (OtherBodyIndex :type Integer) (bFromSweep :type Boolean) (SweepResult :type Hit%20Result%20Structure%20%28by%20ref%29))
  ;[1 1 1] Checks if the player is in range.
  (bind _asvrpawn (Utilities|Casting|CastToVRPawn OtherActor))
  (AI|Components|Blackboard|SetValueasObject (Variables|/Script/AIModule.AIController|GetBlackboard (AI|GetAIController (Pawn|GetController))) (Utilities|Name|MakeLiteralName "TargetActor") _asvrpawn))

(event Custom|SpawnDecal
  (bind _returnvalue (Transformation|GetActorLocation))
  ;[1 1 1] Spawns a blood decal on the location of the zombie where he is hit.
  (bind _outhit (Collision|LineTraceByChannel _returnvalue (- _returnvalue (Variables|Default|GetbloodDirection)) "TraceTypeQuery1" false (Utilities|Array|MakeArray self) "None"))
  (Game|SpawnActorfromClass "/Game/AfterTheFall/ParticleSystems/BloodPuddle/BP_BloodPuddleDecal.BP_BloodPuddleDecal_C" (Math|Conversions|ToTransform(Vector) (.ImpactPoint (Collision|BreakHitResult _outhit))) "Undefined" 0 0))

(event Custom|Attack
  ;[1 1 1] Sent to the animationcontroller to play the attck animation.
  (bind _asabp_zombie_ (Utilities|Casting|CastToABP_Zombie_ (Components|SkeletalMesh|GetAnimInstance (Variables|Character|GetMesh))))
  (Variables|/Game/AfterTheFall/Enemies/ABP_Zombie_.ABP_Zombie__C|SetbAttack _asabp_zombie_ true)
  (Class|AudioParameterControllerInterface|SetTriggerParameter (Variables|Default|GetMS_ZombieSoundEffects) "AttackEffect"))

(event EventTick
  (params (DeltaSeconds :type Float%20%28single-precision%29))
  (bind _mesh (Variables|Character|GetMesh))
  (bind _returnvalue (Transformation|GetSocketLocation _mesh "R_Hand"))
  ;[1 1 1] A sphere around the hand of the zombie. While animation is playing.
  (if (Variables|Default|GetbCheckSphere)
    (bind _outhits (Collision|MultiSphereTraceByChannel _returnvalue _returnvalue (Variables|Default|GetAttackSphereRadius) "TraceTypeQuery1" false 0 "None"))
    (for _array_element _outhits
      (bind _asvrpawn (Utilities|Casting|CastToVRPawn (.HitActor (Collision|BreakHitResult _array_element))))
      (Default|TakeDamage (Variables|/Game/VRTemplate/Blueprints/VRPawn.VRPawn_C|GetAC_HealthComponent _asvrpawn) (Variables|Default|GetDamage))
      (Variables|Default|SetbCheckSphere false))))

(event EventOnHit
  (params (Damage :type Float%20%28double-precision%29) (Impact%20Position :type Vector :default "0, 0, 0") (Rotation :type Rotator :default "0, 0, 0"))
  ;[1 1 1] When the zombie is hit, take away damage. Spawn a decal when the zombie isn't dead.
  (if (Variables|Default|GetbDead)
    _
    (else
      (CallFunction|SpawnDecal)
      (Default|TakeDamage (Variables|Default|GetAC_HealthComponent) Damage)
      ;[1 1 1] Play flinch montage
      (bind _asabp_zombie_ (Utilities|Casting|CastToABP_Zombie_ (Components|SkeletalMesh|GetAnimInstance (Variables|Character|GetMesh))))
      (Animation|Montage|MontagePlay _asabp_zombie_ "/Game/AfterTheFall/Enemies/AM_Zombie_Flinch.AM_Zombie_Flinch" 1.0 "MontageLength" 0.0 true)))
  ;[1 1 1] Start blood particle effect
  (bind _returnvalue (Game|SpawnActorfromClass "/Game/AfterTheFall/ParticleSystems/BP_BloodFX.BP_BloodFX_C" (Math|Transform|MakeTransform Impact%20Position Rotation) "Undefined" 0 0))
  (Components|Activation|Activate (Variables|/Script/Engine.Actor|GetRootComponent _returnvalue) true)
  (Utilities|FlowControl|Delay 3.0)
  (Actor|DestroyActor _returnvalue))

(event EventBeginPlay
  ;[1 1 1] Set the vision sphere of the zombie.
  (Components|Sphere|SetSphereRadius (Variables|Default|GetVisionSphere) (Variables|Default|GetVisionSphereRadius) true))

(fn ConstructionScript)