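; BP_AmmoBox is an ammo box that opens to offer two magazines when its lock is shot or touched by a BP_Pistol.
; A hit within the lock's sphere or a pistol overlap plays the opening animation and audio, disables the lock collider and spawns the magazines.
; After a reset delay, it destroys magazines still flagged as AmmoBoxMagazine, plays the closing animation and re-enables the lock.
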(event OnComponentBeginOverlap(LockCollider)
  (params (OverlappedComponent :type Primitive%20Component%20Object%20Reference) (OtherActor :type Actor%20Object%20Reference) (OtherComp :type Primitive%20Component%20Object%20Reference) (OtherBodyIndex :type Integer) (bFromSweep :type Boolean) (SweepResult :type Hit%20Result%20Structure%20%28by%20ref%29))
  (bind _model (Variables|Default|GetModel))
  (bind _model_2 (Variables|Default|GetModel))
  ;[1 1 1] If the gun is in the sphere collider of the lock, the ammo box will open
  (if (== (Utilities|GetClass OtherActor) "/Game/AfterTheFall/Weapons/BP_Pistol.BP_Pistol_C")
    ;[1 1 1] It will play the opening animation of the ammo box. It disable the collider on the lock and it will spawn in magazines that the player can grab
    (Components|Animation|SetAnimation _model "/Game/AfterTheFall/Models/AmmoBox/AmmoBox_Mesh/AS_AmmoBox2.AS_AmmoBox2")
    (Audio|Components|Audio|Play _model false)
    (Audio|Components|Audio|Play (Variables|Default|GetAmmoBoxAudioSource) 0.0)
    (Collision|SetCollisionEnabled (Variables|Default|GetLockCollider) "NoCollision")
    (CallFunction|SpawninMagazines)
    (Utilities|FlowControl|Delay (Variables|Default|GetAmmoBoxResetTime))
    ;[1 1 1] it destroys the magazine that are still in the ammo box. After that, the closing animation of the ammo box will play and the lock collider will be enabled.
    (CallFunction|DestoryMagazines (Variables|Default|GetFirstMagazine))
    (CallFunction|DestoryMagazines (Variables|Default|GetSecondMagazine))
    (Components|Animation|SetAnimation _model_2 "/Game/AfterTheFall/Models/AmmoBox/AmmoBox_Mesh/AS_AmmoBoxclosing.AS_AmmoBoxclosing")
    (Audio|Components|Audio|Play _model_2 false)
    (Collision|SetCollisionEnabled (Variables|Default|GetLockCollider) "QueryAndPhysics")))

(event EventOnHit
  (params (Damage :type Float%20%28double-precision%29) (Impact%20Position :type Vector :default "0, 0, 0") (Rotation :type Rotator :default "0, 0, 0"))
  (bind _model (Variables|Default|GetModel))
  (bind _model_2 (Variables|Default|GetModel))
  (bind _lockcollider (Variables|Default|GetLockCollider))
  ;[1 1 1] Check if the position of the raycast hit is in the sphere collider of the lock collider
  (if (and (<= (Math|Vector|Distance(Vector) Impact%20Position (Transformation|GetWorldLocation _lockcollider)) (+ (Variables|/Script/Engine.SphereComponent|GetSphereRadius _lockcollider) 1.0)) (Class|PrimitiveComponent|IsCollisionEnabled (Variables|Default|GetLockCollider)))
    ;[1 1 1] It will play the opening animation of the ammo box. It disable the collider on the lock and it will spawn in magazines that the player can grab
    (Components|Animation|SetAnimation _model "/Game/AfterTheFall/Models/AmmoBox/AmmoBox_Mesh/AS_AmmoBox2.AS_AmmoBox2")
    (Audio|Components|Audio|Play _model false)
    (Audio|Components|Audio|Play (Variables|Default|GetAmmoBoxAudioSource) 0.0)
    (Collision|SetCollisionEnabled (Variables|Default|GetLockCollider) "NoCollision")
    (CallFunction|SpawninMagazines)
    (Utilities|FlowControl|Delay (Variables|Default|GetAmmoBoxResetTime))
    ;[1 1 1] it destroys the magazine that are still in the ammo box. After that, the closing animation of the ammo box will play and the lock collider will be enabled.
    (CallFunction|DestoryMagazines (Variables|Default|GetFirstMagazine))
    (CallFunction|DestoryMagazines (Variables|Default|GetSecondMagazine))
    (Components|Animation|SetAnimation _model_2 "/Game/AfterTheFall/Models/AmmoBox/AmmoBox_Mesh/AS_AmmoBoxclosing.AS_AmmoBoxclosing")
    (Audio|Components|Audio|Play _model_2 false)
    (Collision|SetCollisionEnabled (Variables|Default|GetLockCollider) "QueryAndPhysics")))

(fn ConstructionScript)

(fn SpawninMagazines
  (bind _returnvalue (Game|SpawnActorfromClass "/Game/AfterTheFall/Weapons/BP_Magazine.BP_Magazine_C" (Transformation|GetWorldTransform (Variables|Default|GetFirstMagazineSpawnLocation)) "Undefined" 0 0))
  (bind _output_get (Variables|Default|SetFirstMagazine _returnvalue))
  (Variables|/Game/AfterTheFall/Weapons/BP_Magazine.BP_Magazine_C|SetAmmoBoxMagazine _output_get true)
  (bind _returnvalue_2 (Game|SpawnActorfromClass "/Game/AfterTheFall/Weapons/BP_Magazine.BP_Magazine_C" (Transformation|GetWorldTransform (Variables|Default|GetSecondMagazineSpawnLocation)) "Undefined" 0 0))
  (bind _output_get_2 (Variables|Default|SetSecondMagazine _returnvalue_2))
  (Variables|/Game/AfterTheFall/Weapons/BP_Magazine.BP_Magazine_C|SetAmmoBoxMagazine _output_get_2 true))

(fn DestoryMagazines
  (params (Magazine :type BP%20Magazine%20Object%20Reference))
  (Utilities|IsValid Magazine
    (:Is%20Valid
      (if (Variables|/Game/AfterTheFall/Weapons/BP_Magazine.BP_Magazine_C|GetAmmoBoxMagazine Magazine)
        (Actor|DestroyActor Magazine))
      (return))))