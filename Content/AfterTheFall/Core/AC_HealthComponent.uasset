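; Health component for After the Fall that tracks an owner's health and death state.
; Health starts at the start value on BeginPlay, and TakeDamage subtracts the absolute damage while the owner is alive.
; Damage and death are broadcast through event dispatchers, with a Dead flag blocking further hits.
; GetHealthPercent returns current health as an unclamped fraction of the start value.
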(event Custom|TakeDamage
  (params (Damage :type Float%20%28double-precision%29))
  (bind _returnvalue (Math|Float|Absolute(Float) Damage))
  ;[1 1 1] TakeDamage
  (if (not (Variables|Default|GetbDead))
    (bind _output_get (Variables|Default|SetCurrentHealth (- (Variables|Default|GetCurrentHealth) _returnvalue)))
    (Default|CallOnDamage _output_get _returnvalue)
    (if (<= _output_get 0.0)
      (Default|CallOnDeath)
      (Variables|Default|SetbDead true))))

(event EventBeginPlay
  (Variables|Default|SetCurrentHealth (Variables|Default|GetStartHealth)))

(fn GetHealthPercent
  (return (/ (Variables|Default|GetCurrentHealth) (Variables|Default|GetStartHealth))))