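; Walking sound effect Blueprint that starts and stops footstep audio based on whether a supplied velocity is non-zero.
; PlayWalkAudio, intended for per-tick calls, passes StepsPerMinute to the WalkingSound audio component and uses trigger parameters to signal walking or stopping.
; The IsWalkingAudioPlaying flag keeps the start trigger from refiring, while the stop trigger repeats whenever velocity is zero.
; The event graph holds only unconnected test calls that never run.
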(fn ConstructionScript)

(fn PlayWalkAudio
  (params (Velocity :type Vector) (StepsPerMinute :type Integer))
  (bind _walkingsound (Variables|Default|GetWalkingSound))
  ;[1 1 1] Play Walk Audio - Play a sound when player is moving, StepsPerMinute is the time between each step
  (Effects|Components|ParticleSystem|SetIntParameter (Variables|Default|GetWalkingSound) "StepsPerMinute" StepsPerMinute)
  (if (Math|Vector|VectorIsZero Velocity)
    (Class|AudioParameterControllerInterface|SetTriggerParameter _walkingsound "StoppedWalking")
    (Variables|Default|SetIsWalkingAudioPlaying false)
    (elif (not (Variables|Default|GetIsWalkingAudioPlaying))
      (Class|AudioParameterControllerInterface|SetTriggerParameter _walkingsound "IsWalking")
      (Variables|Default|SetIsWalkingAudioPlaying true))))