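; Audio component that drives a grenade's countdown beeps and explosion cue through a supplied MetaSound.
; SetupEvent stores the timing settings; PlayGrenadeDetonation counts down with delta time and triggers each beep.
; After a set number of evenly spaced beeps, UpdateDelayTillBeep shrinks each interval by a degrade rate for an accelerating warning.
; Below a short threshold it fires the CountDownFinished trigger, deactivates and returns true.
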(fn SetupEvent
  (params (activateGrenade :type Boolean) (totalBeepsBeforeDetonation :type Integer) (delayBetweenBeep :type Float%20%28double-precision%29) (detonationDelayTillBeep :type Float%20%28double-precision%29) (detonationDegradeRate :type Float%20%28double-precision%29) (metaSoundSource :type Audio%20Parameter%20Controller%20Interface%20Interface))
  ;[1 0.1834 0.5895] All the given data for the grenade is setup
  (Variables|Default|SetgrenadeActivated activateGrenade)
  (Variables|Default|SettotalBeepsBeforeDetonation totalBeepsBeforeDetonation)
  (Variables|Default|SetdelayTillBeep delayBetweenBeep)
  (Variables|Default|SetnewDelayTillBeep detonationDelayTillBeep)
  (Variables|Default|SetdegradeRate detonationDegradeRate)
  (Variables|Default|SetgrenadeMetaSound metaSoundSource))

(fn PlayGrenadeDetonation
  (params (deltaSeconds :type Float%20%28double-precision%29))
  ;[1 1 1] Play beep sound when timer hits 0
  (Variables|Default|SetdeltaSeconds deltaSeconds)
  (if (Variables|Default|GetgrenadeActivated)
    (bind _output_get (Variables|Default|SetdelayTillBeep (- (Variables|Default|GetdelayTillBeep) (Variables|Default|GetdeltaSeconds))))
    (Math|Float|CompareFloat _output_get 0.0
      (:==
        _)
      (:<
        _))
    (Class|AudioParameterControllerInterface|SetTriggerParameter (Variables|Default|GetgrenadeMetaSound) "PlayCountDownBeep")
    (if (Variables|Default|GetdetonationActivated)
      ;[1 1 1] Degrees the delay time after each beep. When this time is below a specific threshold, play the explosion SFX
      (bind _calculatedtime (CallFunction|UpdateDelayTillBeep (Variables|Default|GetnewDelayTillBeep) (Variables|Default|GetdeltaSeconds) (Variables|Default|GetdegradeRate)))
      (bind _output_get_2 (Variables|Default|SetnewDelayTillBeep _calculatedtime))
      (bind _output_get_3 (Variables|Default|SetdelayTillBeep _output_get_2))
      (Math|Float|CompareFloat _output_get_3 0.1
        (:<
          (Class|AudioParameterControllerInterface|SetTriggerParameter (Variables|Default|GetgrenadeMetaSound) "CountDownFinished")
          (Variables|Default|SetdetonationActivated false)
          (Variables|Default|SetgrenadeActivated false)
          (Variables|Default|SetcurrentHeardBeepsAmount 0)
          (return true)))
      (else
        ;[1 1 1] Reset time after a beep has been heard and the total amount of beeps hasn't been passed
        (Math|Integer|CompareInt (Variables|Default|GetcurrentHeardBeepsAmount) (Variables|Default|GettotalBeepsBeforeDetonation)
          (:>
            (Variables|Default|SetdetonationActivated true :!label _label))
          (:==
            (goto _label))
          (:<
            (Variables|Default|SetcurrentHeardBeepsAmount (+ (Variables|Default|GetcurrentHeardBeepsAmount) 1))
            (Variables|Default|SetdelayTillBeep (Variables|Default|GetnewDelayTillBeep))))))))

(fn UpdateDelayTillBeep
  (params (time :type Float%20%28double-precision%29) (deltaSeconds :type Float%20%28double-precision%29) (degradeRate :type Float%20%28double-precision%29))
  ;[1 1 1] Degrade the time between each beep sound, creating that iconic "before detonation" sound
  (return (* (- time deltaSeconds) degradeRate)))