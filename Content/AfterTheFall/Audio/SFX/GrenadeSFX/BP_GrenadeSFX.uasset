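; Grenade sound actor that plays a MetaSound beep countdown and detonation through BPGrenadeSFXComponent.
; Space bar arms the component with the beep count, timing and MetaSound, and Tick drives its detonation update.
; The actor also holds its own countdown functions, not called in this graph, that fire MetaSound triggers and shorten each beep interval until a finish trigger.
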(event EventTick
  (params (DeltaSeconds :type Float%20%28single-precision%29))
  (Default|PlayGrenadeDetonation (Variables|Default|GetBP_GrenadeSFX_Component) DeltaSeconds))

(event EventBeginPlay
  (Input|EnableInput (Game|GetPlayerController 0)))

(event Input|KeyboardEvents|SpaceBar
  (params (Key :type Key%20Structure))
  (:Pressed
    (Default|SetupEvent (Variables|Default|GetBP_GrenadeSFX_Component) true 4 1.0 1.0 0.0 (Variables|Default|GetMS_GrenadeSound))))

(fn ConstructionScript)

(fn PlayGrenadeDetonationEvent
  (params (grenadeActivated :type Boolean) (deltaSeconds :type Float%20%28double-precision%29) (timeTillExplosion :type Float%20%28double-precision%29))
  (if grenadeActivated
    (bind _output_get (Variables|Default|SetCurrent%20Delay%20Between%20Beep (- (Variables|Default|GetCurrent%20Delay%20Between%20Beep) deltaSeconds)))
    (Math|Float|CompareFloat _output_get 0.0
      (:==
        _)
      (:<
        _))
    (Class|AudioParameterControllerInterface|SetTriggerParameter (Variables|Default|GetMS_GrenadeSound) "PlayCountDownBeep")
    (bind _new_calculated_delay (CallFunction|UpdateCurrentDelay (Variables|Default|GetNew%20Delay%20Between%20Beep) deltaSeconds))
    (bind _output_get_2 (Variables|Default|SetCurrent%20Delay%20Between%20Beep _new_calculated_delay))
    (Math|Float|CompareFloat _output_get_2 0.0
      (:==
        _)
      (:<
        _))
    (Variables|Default|SetGrenateActivated false)
    (Variables|Default|SetNew%20Delay%20Between%20Beep 1.0)
    (Class|AudioParameterControllerInterface|SetTriggerParameter (Variables|Default|GetMS_GrenadeSound) "CountDownFinished")))

(fn UpdateCurrentDelay
  (params (Delay%20Between%20Beep :type Float%20%28double-precision%29) (Delta%20Seconds :type Float%20%28double-precision%29))
  (bind _output_get (Variables|Default|SetNew%20Delay%20Between%20Beep (* (- Delay%20Between%20Beep Delta%20Seconds) 0.9)))
  (return _output_get))